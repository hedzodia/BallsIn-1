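; BP_Spawner is a respawn point that spawns a ThirdPersonCharacter for its linked player controller.
; While Spect is true, Tick checks every frame whether that controller's pawn is invalid.
; If so, after a short Delay it spawns a character at the spawner's transform, has the controller possess it, then assigns the spawner's TeamID to it.
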(event Custom|spawnIsDead
  (Utilities|IsValid (Pawn|GetControlledPawn (Variables|Default|GetlinkedPC))
    (:Is%20Not%20Valid
      (Utilities|FlowControl|Delay 1.0)
      (bind _returnvalue (Game|SpawnActorfromClass "/Game/Blueprints/team/ThirdPersonCharacter.ThirdPersonCharacter_C" (Transformation|GetActorTransform) "Undefined" 0 0))
      (Pawn|Possess (Variables|Default|GetlinkedPC) _returnvalue)
      (Variables|/Game/Blueprints/team/ThirdPersonCharacter.ThirdPersonCharacter_C|SetteamId _returnvalue (Variables|Default|GetTeamID)))))

(event EventTick
  (params (DeltaSeconds :type Float%20%28single-precision%29))
  (if (Variables|Default|GetSpect)
    (CallFunction|SpawnIsDead)))

(fn ConstructionScript)