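; Energy ball pickup that a ThirdPersonCharacter collects by overlapping its sphere, giving that character the energetique state.
; On overlap, if the character lacks that state, it sets IsEnergetique, shows the character's particle system, disables its own collision and snaps the sphere to the left-hand socket.
; Tick polls the overlapped character and, once the flag is false, destroys the ball and hides the particles.
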(event OnComponentBeginOverlap(Sphere)
  (params (OverlappedComponent :type Primitive%20Component%20Object%20Reference) (OtherActor :type Actor%20Object%20Reference) (OtherComp :type Primitive%20Component%20Object%20Reference) (OtherBodyIndex :type Integer) (bFromSweep :type Boolean) (SweepResult :type Hit%20Result%20Structure%20%28by%20ref%29))
  (bind _asthird_person_character (Utilities|Casting|CastToThirdPersonCharacter OtherActor))
  (if (not (Variables|/Game/Blueprints/team/ThirdPersonCharacter.ThirdPersonCharacter_C|GetisEnergetique? _asthird_person_character))
    (Variables|/Game/Blueprints/team/ThirdPersonCharacter.ThirdPersonCharacter_C|SetisEnergetique? _asthird_person_character true)
    (Rendering|SetVisibility (Variables|/Game/Blueprints/team/ThirdPersonCharacter.ThirdPersonCharacter_C|GetParticleSystem _asthird_person_character) true false)
    (Collision|SetActorEnableCollision false)
    (Transformation|AttachComponentToComponent (Variables|Default|GetSphere) (Variables|/Script/Engine.Character|GetMesh _asthird_person_character) "hand_l" "SnapToTarget" "KeepRelative" "KeepRelative" false)))

(event EventTick
  (params (DeltaSeconds :type Float%20%28single-precision%29))
  (bind _asthird_person_character (Utilities|Casting|CastToThirdPersonCharacter (stale OnComponentBeginOverlap(Sphere) OtherActor)))
  (if (not (Variables|/Game/Blueprints/team/ThirdPersonCharacter.ThirdPersonCharacter_C|GetisEnergetique? _asthird_person_character))
    (Actor|DestroyActor)
    (Rendering|SetVisibility (Variables|/Game/Blueprints/team/ThirdPersonCharacter.ThirdPersonCharacter_C|GetParticleSystem _asthird_person_character) false false)))

(fn ConstructionScript)