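; Goal actor that holds a team color and detects balls overlapping it.
; SetTeamColor stores the color, and the overlap event casts the other actor to BP_Ball to compare RGB channels with the ball's color, ignoring alpha.
; Both outcomes of the comparison are empty, so the only visible result is a debug print of the two colors, with no scoring logic.
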(event Custom|SetTeamColor
  (params (InLinearColor :type Linear%20Color%20Structure))
  (Variables|Default|SetColor InLinearColor))

(event Collision|EventActorBeginOverlap
  (params (OtherActor :type Actor%20Object%20Reference))
  (bind _color (Variables|Default|Getcolor))
  (bind _asbp_ball (Utilities|Casting|CastToBP_Ball OtherActor))
  (if (Math|Boolean|ORBoolean (!= (.r _color) (.r (Variables|/Game/Blueprints/BP_Ball.BP_Ball_C|Getcolor _asbp_ball))) (!= (.g _color) (.g (Variables|/Game/Blueprints/BP_Ball.BP_Ball_C|Getcolor _asbp_ball))) (!= (.b _color) (.b (Variables|/Game/Blueprints/BP_Ball.BP_Ball_C|Getcolor _asbp_ball))))
    _
    (else
      _))
  (Development|PrintString (Utilities|String|Append (Utilities|String|ToString(Integer) (Variables|Default|Getcolor)) (Utilities|String|ToString(Integer) (Variables|/Game/Blueprints/BP_Ball.BP_Ball_C|Getcolor _asbp_ball)))))

(fn ConstructionScript)