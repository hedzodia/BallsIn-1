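; BP_Ball is a team ball that takes on the team of the last character it hits and scores in the opposing goal.
; On hit, it copies the ThirdPersonCharacter's TeamId, recolors its sphere material and switches to that team's collision object type.
; BeginPlay caches both Goal actors by team.
; Overlapping another team's goal increments Score on the ball team's own Goal, then destroys the ball.
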(event Collision|EventActorBeginOverlap
  (params (OtherActor :type Actor%20Object%20Reference))
  (bind _goal1 (Variables|Default|Getgoal1))
  (bind _goal2 (Variables|Default|Getgoal2))
  ;[1 1 1] Score
  (bind _asgoal (Utilities|Casting|CastToGoal OtherActor))
  (if (!= (Variables|Default|GetteamId) (Variables|/Game/Blueprints/Goal/Goal.Goal_C|Getteam _asgoal))
    (if (== (Variables|Default|GetteamId) 1)
      (Variables|/Game/Blueprints/Goal/Goal.Goal_C|Setscore _goal1 (+ 1 (Variables|/Game/Blueprints/Goal/Goal.Goal_C|Getscore _goal1)))
      (Actor|DestroyActor :!label _label)
      (elif (== (Variables|Default|GetteamId) 2)
        (Variables|/Game/Blueprints/Goal/Goal.Goal_C|Setscore _goal2 (+ 1 (Variables|/Game/Blueprints/Goal/Goal.Goal_C|Getscore _goal2)))
        (goto _label)))))

(event Collision|EventHit
  (params (MyComp :type Primitive%20Component%20Object%20Reference) (Other :type Actor%20Object%20Reference) (OtherComp :type Primitive%20Component%20Object%20Reference) (bSelfMoved :type Boolean) (HitLocation :type Vector :default "0, 0, 0") (HitNormal :type Vector :default "0, 0, 0") (NormalImpulse :type Vector :default "0, 0, 0") (Hit :type Hit%20Result%20Structure%20%28by%20ref%29))
  (bind _asthird_person_character (Utilities|Casting|CastToThirdPersonCharacter Other))
  (Variables|Default|SetteamId (Variables|/Game/Blueprints/team/ThirdPersonCharacter.ThirdPersonCharacter_C|GetteamId _asthird_person_character))
  ;[1 1 1] color&collision
  (Rendering|Material|SetVectorParameterValueonMaterials (Variables|Default|GetSphere) "Color" (Math|Conversions|ToVector(LinearColor) (Variables|/Game/Blueprints/team/ThirdPersonCharacter.ThirdPersonCharacter_C|GetColor _asthird_person_character)))
  (if (== (Variables|Default|GetteamId) 1)
    (Collision|SetCollisionObjectType (Variables|Default|GetSphere) "ECC_GameTraceChannel1")
    (elif (== (Variables|Default|GetteamId) 2)
      (Collision|SetCollisionObjectType (Variables|Default|GetSphere) "ECC_GameTraceChannel2"))))

(event EventBeginPlay
  ;[1 1 1] Score
  (bind _outactors (Actor|GetAllActorsOfClass "/Game/Blueprints/Goal/Goal.Goal_C"))
  (for _array_element _outactors
    (if (== (Variables|/Game/Blueprints/Goal/Goal.Goal_C|Getteam _array_element) 1)
      (Variables|Default|Setgoal1 _array_element)
      (elif (== (Variables|/Game/Blueprints/Goal/Goal.Goal_C|Getteam _array_element) 2)
        (Variables|Default|Setgoal2 _array_element)))))

(fn ConstructionScript)