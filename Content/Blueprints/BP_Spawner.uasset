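; BP_Spawner is an actor that respawns a player's character when their controller has no valid pawn.
; While the Spect flag is set, Tick runs a check on the LinkedPC controller every frame.
; If no valid pawn is controlled, it spawns a ThirdPersonCharacter at the spawner's transform and has LinkedPC possess it.
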(event Custom|spawnIsDead
  (Utilities|IsValid (Pawn|GetControlledPawn (Variables|Default|GetlinkedPC))
    (:Is%20Not%20Valid
      (bind _returnvalue (Game|SpawnActorfromClass "/Game/Blueprints/ThirdPersonCharacter.ThirdPersonCharacter_C" (Transformation|GetActorTransform) "Undefined" 0 0))
      (Pawn|Possess (Variables|Default|GetlinkedPC) _returnvalue))))

(event EventTick
  (params (DeltaSeconds :type Float%20%28single-precision%29))
  (if (Variables|Default|GetSpect)
    (CallFunction|SpawnIsDead)))

(fn ConstructionScript)