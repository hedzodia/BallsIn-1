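; Capture zone for two teams: a tug-of-war value from -100 to 100 decides which team owns its walls and platform.
; Overlaps count players per team; Tick shifts the value toward a team alone inside and freezes it when contested.
; An energized character instantly captures the zone unless already owned, spending its energy and ball.
; Past the halfway thresholds, walls and platform take the owner's color and switch collision channels so only that team overlaps them.
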(event Custom|capture
  (bind _eventtick (Variables|Default|GeteventTick))
  (bind _returnvalue (* _eventtick 2e+01))
  ;[1 1 1] capture
  (if (not (and (> (Variables|Default|GetnbTeam1) 0) (> (Variables|Default|GetnbTeam2) 0)))
    (if (== 1 (Variables|Default|Getteam1))
      (if (not (== (Variables|Default|Get%25capture) 1e+02))
        (Variables|Default|Set%25capture (+ (Variables|Default|Get%25capture) _returnvalue)))
      (elif (== (Variables|Default|Getteam2) 2)
        (if (not (== (Variables|Default|Get%25capture) -1e+02))
          (Variables|Default|Set%25capture (- (Variables|Default|Get%25capture) _returnvalue)))))))

(event Custom|ColorCube
  ;[1 1 1] color
  (Rendering|Components|TextRender|SetText (Variables|Default|GetTextRender) (Utilities|Text|ToText(Float) (Variables|Default|Get%25capture) "HalfToEven"))
  (for _array_element (Variables|Default|Getmur)
    (if (< (Variables|Default|Get%25capture) -5e+01)
      (Rendering|Material|SetVectorParameterValueonMaterials (Variables|/Game/Blueprints/Zone/Mur.Mur_C|GetCube _array_element) "Color" (Math|Conversions|ToVector(LinearColor) (Variables|Default|Getcolor2)))
      (Collision|SetCollisionResponsetoChannel (Variables|/Game/Blueprints/Zone/Mur.Mur_C|GetCube _array_element) "ECC_GameTraceChannel2" "ECR_Overlap")
      (Collision|SetCollisionResponsetoChannel (Variables|/Game/Blueprints/Zone/Mur.Mur_C|GetCube _array_element) "ECC_GameTraceChannel1" "ECR_Block")
      (elif (> (Variables|Default|Get%25capture) 5e+01)
        (Rendering|Material|SetVectorParameterValueonMaterials (Variables|/Game/Blueprints/Zone/Mur.Mur_C|GetCube _array_element) "Color" (Math|Conversions|ToVector(LinearColor) (Variables|Default|Getcolor1)))
        (Collision|SetCollisionResponsetoChannel (Variables|/Game/Blueprints/Zone/Mur.Mur_C|GetCube _array_element) "ECC_GameTraceChannel1" "ECR_Overlap")
        (Collision|SetCollisionResponsetoChannel (Variables|/Game/Blueprints/Zone/Mur.Mur_C|GetCube _array_element) "ECC_GameTraceChannel2" "ECR_Block")
        (else
          (Rendering|Material|SetVectorParameterValueonMaterials (Variables|/Game/Blueprints/Zone/Mur.Mur_C|GetCube _array_element) "Color" "1.000000,1.000000,1.000000")
          (Collision|SetCollisionResponsetoChannel (Variables|/Game/Blueprints/Zone/Mur.Mur_C|GetCube _array_element) "ECC_GameTraceChannel1" "ECR_Block")
          (Collision|SetCollisionResponsetoChannel (Variables|/Game/Blueprints/Zone/Mur.Mur_C|GetCube _array_element) "ECC_GameTraceChannel2" "ECR_Block"))))))

(event Collision|EventActorBeginOverlap
  (params (OtherActor :type Actor%20Object%20Reference))
  ;[1 1 1] overlap
  (bind _asthird_person_character (Utilities|Casting|CastToThirdPersonCharacter OtherActor))
  ;;[1 1 1] color&team&energie
  (if (== (Variables|/Game/Blueprints/team/ThirdPersonCharacter.ThirdPersonCharacter_C|GetteamId _asthird_person_character) 1)
    (Variables|Default|Setcolor1 (Variables|/Game/Blueprints/team/ThirdPersonCharacter.ThirdPersonCharacter_C|GetColor _asthird_person_character))
    (Variables|Default|Setteam1 (Variables|/Game/Blueprints/team/ThirdPersonCharacter.ThirdPersonCharacter_C|GetteamId _asthird_person_character))
    (Variables|Default|SetnbTeam1 (+ (Variables|Default|GetnbTeam1) 1))
    (if (Variables|/Game/Blueprints/team/ThirdPersonCharacter.ThirdPersonCharacter_C|GetisEnergetique? _asthird_person_character)
      (if (< (Variables|Default|Get%25capture) 5e+01)
        (Variables|Default|Set%25capture 99.0)
        (Variables|/Game/Blueprints/team/ThirdPersonCharacter.ThirdPersonCharacter_C|SetisEnergetique? _asthird_person_character false :!label _label)
        (Rendering|SetVisibility (Variables|/Game/Blueprints/team/ThirdPersonCharacter.ThirdPersonCharacter_C|GetParticleSystem _asthird_person_character) false false)
        (Actor|DestroyActor (Variables|/Game/Blueprints/team/ThirdPersonCharacter.ThirdPersonCharacter_C|GettargetBall _asthird_person_character))))
    (elif (== (Variables|/Game/Blueprints/team/ThirdPersonCharacter.ThirdPersonCharacter_C|GetteamId _asthird_person_character) 2)
      (Variables|Default|Setcolor2 (Variables|/Game/Blueprints/team/ThirdPersonCharacter.ThirdPersonCharacter_C|GetColor _asthird_person_character))
      (Variables|Default|Setteam2 (Variables|/Game/Blueprints/team/ThirdPersonCharacter.ThirdPersonCharacter_C|GetteamId _asthird_person_character))
      (Variables|Default|SetnbTeam2 (+ (Variables|Default|GetnbTeam2) 1))
      (if (Variables|/Game/Blueprints/team/ThirdPersonCharacter.ThirdPersonCharacter_C|GetisEnergetique? _asthird_person_character)
        (if (> (Variables|Default|Get%25capture) -5e+01)
          (Variables|Default|Set%25capture -99.0)
          (goto _label))))))

(event EventTick
  (params (DeltaSeconds :type Float%20%28single-precision%29))
  ;[1 1 1] event Tick
  (Variables|Default|SeteventTick DeltaSeconds)
  (if (and (<= (Variables|Default|Get%25capture) 1e+02) (>= (Variables|Default|Get%25capture) -1e+02))
    (CallFunction|Capture)
    (CallFunction|ColorCube)
    (elif (< (Variables|Default|Get%25capture) -1e+02)
      (Variables|Default|Set%25capture -1e+02)
      (elif (> (Variables|Default|Get%25capture) 1e+02)
        (Variables|Default|Set%25capture 1e+02)))))

(event Collision|EventActorEndOverlap
  (params (OtherActor :type Actor%20Object%20Reference))
  ;[1 1 1] overlap
  (bind _asthird_person_character (Utilities|Casting|CastToThirdPersonCharacter OtherActor))
  (if (== (Variables|/Game/Blueprints/team/ThirdPersonCharacter.ThirdPersonCharacter_C|GetteamId _asthird_person_character) (Variables|Default|Getteam1))
    (bind _output_get (Variables|Default|SetnbTeam1 (- (Variables|Default|GetnbTeam1) 1)))
    (if (== _output_get 0)
      (Variables|Default|Setteam1 0))
    (elif (== (Variables|/Game/Blueprints/team/ThirdPersonCharacter.ThirdPersonCharacter_C|GetteamId _asthird_person_character) (Variables|Default|Getteam2))
      (bind _output_get_2 (Variables|Default|SetnbTeam2 (- (Variables|Default|GetnbTeam2) 1)))
      (if (== _output_get_2 0)
        (Variables|Default|Setteam2 0)))))

(fn ConstructionScript)